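; Game mode that handles single-slot saving and loading of the player's position and inventory.
; On BeginPlay it restores the first-person character's transform and the game instance's inventory data from the "save1" slot, or creates an empty save if none exists.
; SaveGame writes both values back to that slot, while LoadGame simply restarts the level so BeginPlay reapplies the saved state.
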(event `self.ReceiveBeginPlay`
  (bind _returnvalue (`GameplayStatics.DoesSaveGameExist` "save1"))
  (if _returnvalue
    ;[1 1 1] Load Game
    (bind _returnvalue_2 (`GameplayStatics.LoadGameFromSlot` "save1"))
    ;;[1 1 1] Load Player Transform
    (bind _asbp_save_game (cast `/Game/Blueprints/BP_SaveGame` _returnvalue_2))
    (bind _asfirst_person_character (cast `/Game/Characters/FirstPersonBP/Blueprints/FirstPersonCharacter` (`GameplayStatics.GetPlayerCharacter` 0)))
    (`SceneComponent.K2_SetWorldTransform` (`Actor.RootComponent` _asfirst_person_character) (`/Game/Blueprints/BP_SaveGame.Transform` _asbp_save_game) false true)
    ;;[1 1 1] Load Inventory Data
    (bind _asbp_save_game_2 (cast `/Game/Blueprints/BP_SaveGame` _returnvalue_2))
    (set `/Game/Blueprints/DunsteelGameInstance.InventoryData` (`/Game/Blueprints/BP_SaveGame.InventoryData` _asbp_save_game_2) (cast `/Game/Blueprints/DunsteelGameInstance` (`GameplayStatics.GetGameInstance`) :!pure true))
    (else
      ;[1 1 1] Create Save File
      (bind _returnvalue_3 (`GameplayStatics.CreateSaveGameObject` "/Game/Blueprints/BP_SaveGame.BP_SaveGame_C"))
      (`GameplayStatics.SaveGameToSlot` _returnvalue_3 "save1"))))

(event `Load Game`
  ;[1 1 1] LoadGame
  (`KismetSystemLibrary.ExecuteConsoleCommand` "RestartLevel" null))

(event `SaveGame`
  ;[1 1 1] Save Game Info
  (bind _returnvalue (`GameplayStatics.LoadGameFromSlot` "save1"))
  (bind _asbp_save_game (cast `/Game/Blueprints/BP_SaveGame` _returnvalue))
  (set `/Game/Blueprints/BP_SaveGame.Transform` (`self.GetTransform` (cast `/Game/Characters/FirstPersonBP/Blueprints/FirstPersonCharacter` (`GameplayStatics.GetPlayerCharacter` 0) :!pure true)) _asbp_save_game)
  (set `/Game/Blueprints/BP_SaveGame.InventoryData` (`/Game/Blueprints/DunsteelGameInstance.InventoryData` (cast `/Game/Blueprints/DunsteelGameInstance` (`GameplayStatics.GetGameInstance`) :!pure true)) _asbp_save_game)
  (`GameplayStatics.SaveGameToSlot` _asbp_save_game "save1"))

(fn `UserConstructionScript`)