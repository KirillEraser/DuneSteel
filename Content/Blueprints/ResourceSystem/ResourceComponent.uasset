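; Resource component that turns its owning actor into a harvestable node, damaged by tools and destroyed when its health runs out.
; Incoming damage is scaled by a per-tool multiplier looked up from the damage type's tool type.
; Non-lethal hits with a multiplier of at least one spawn a resource above the owner, named by a weighted random pick from the Resources map.
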(event `self.ReceiveBeginPlay`
  (add `Actor.OnTakeAnyDamage` (`self.GetOwner`) (delegate `DamageResource`)))

(event `DamageResource`
  (params (DamagedActor :type "Actor Object Reference") (Damage :type "Float (double-precision)") (DamageType :type "DamageType Object Reference") (InstigatedBy :type "Controller Object Reference") (DamageCauser :type "Actor Object Reference"))
  (bind (_returnvalue_x _returnvalue_y _returnvalue_z) (`KismetMathLibrary.BreakVector` (`Actor.K2_GetActorLocation` (`self.GetOwner`))))
  (`|ExecutionSequence`
    (:`then_0`
      ;[1 1 1] Find a tool which player is hitting with
      (bind _tool (message `/Game/Blueprints/ResourceSystem/Tools/ToolInterface.GetToolType` DamageType))
      (`KismetSystemLibrary.PrintString` (`KismetStringLibrary.Concat_StrStr` "ToolType_Used: " (`|GetEnumeratorNameAsString` _tool)) true true (struct :`R` 1.0 :`G` 0.57309 :`B` 0.039091 :`A` 1.0)))
    (:`then_1`
      (bind _value (`BlueprintMapLibrary.Map_Find` (`self.ToolDamage`) _tool))
      ;[1 1 1] Subtract damage from health
      (set `self.Health` (- (`self.Health`) (* Damage _value)))
      ;[1 1 1] Deletes resource when it runs out of health
      (if (<= (`self.Health`) 0.0)
        (`Actor.K2_DestroyActor` (`self.GetOwner`))
        (else
          ;[1 1 1] Check if enough damage has
          ; been dealt
          (if (>= _value 1.0)
            ;[1 1 1] Drop resource
            (bind _class (`self.DropResource`))
            (`|SpawnActorFromClass` "/Game/Blueprints/ResourceSystem/Resource.Resource_C" (`KismetMathLibrary.MakeTransform` (`KismetMathLibrary.MakeVector` _returnvalue_x _returnvalue_y (+ _returnvalue_z 150.0))) "AdjustIfPossibleButAlwaysSpawn" "OverrideRootScale" null _class null)))))))

(fn `DropResource`
  (returns (Class :type Name))
  (locals (L_Sum :type "Float (double-precision)") (L_RandomNumber :type "Float (double-precision)" :default 0.0))
  (`|ExecutionSequence`
    (:`then_0`
      (bind _values (`BlueprintMapLibrary.Map_Values` (`self.Resources`)))
      (for _array_element _values
        (set `local.L_Sum` (+ _array_element (`local.L_Sum`)))))
    (:`then_1`
      (set `local.L_RandomNumber` (`KismetMathLibrary.RandomFloatInRange` 0.0 (`local.L_Sum`)))
      (bind _keys (`BlueprintMapLibrary.Map_Keys` (`self.Resources`)))
      (for _array_element_2 _keys
        (bind _value (`BlueprintMapLibrary.Map_Find` (`self.Resources`) _array_element_2))
        (if (< (`local.L_RandomNumber`) _value)
          (return _array_element_2)
          (else
            (set `local.L_RandomNumber` (- (`local.L_RandomNumber`) _value))))))))